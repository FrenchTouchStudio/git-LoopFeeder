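; Base projectile actor for the player damage system, with configurable speed, scale, range, effects, sounds and optional homing.
; Construction sets up ProjectileMovement and homing; BeginPlay ignores the owner for collision, plays launch effects and aims velocity at any valid Target.
; A box hit fires the projectile impact call, spawns impact effects and destroys the actor after a short delay.
; Tick destroys the projectile once it reaches MaxRange from its start location.
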(event OnComponentHit(BoxCollision)
  (params (HitComponent :type Primitive%20Component%20Object%20Reference) (OtherActor :type Actor%20Object%20Reference) (OtherComp :type Primitive%20Component%20Object%20Reference) (NormalImpulse :type Vector :default "0, 0, 0") (Hit :type Hit%20Result%20Structure%20%28by%20ref%29))
  (bind _location (Collision|BreakHitResult Hit))
  (Default|CallOnProjectileImpact OtherActor Hit)
  (Effects|SpawnEmitteratLocation (Variables|Effects|GetImpactEffect) _location "0, 0, 0" (Variables|Effects|GetImpactEffectScale))
  (Audio|PlaySoundatLocation (Variables|Sounds|GetImpactSound) _location "0, 0, 0" 1.0 1.0 0.0 0 0 0 0)
  (Utilities|FlowControl|Delay 0.2)
  (Actor|DestroyActor))

(event Custom|RotateToTarget
  (Variables|/Script/Engine.MovementComponent|SetVelocity (Variables|Default|GetProjectileMovement) (* (Math|Vector|GetUnitDirection(Vector) (Transformation|GetActorLocation) (Transformation|GetActorLocation (Variables|Target|GetTarget))) (Variables|ProjectilesSettings|GetSpeed))))

(event EventBeginPlay
  (bind _returnvalue (Components|GetOwner))
  (Development|PrintString (Utilities|GetDisplayName _returnvalue))
  (Collision|IgnoreActorwhenMoving (Variables|Default|GetBoxCollision) _returnvalue true)
  (Effects|SpawnEmitteratLocation (Variables|Effects|GetLaunchEffect) (Transformation|GetWorldLocation (Variables|Default|GetBoxCollision)))
  (Audio|PlaySoundatLocation (Variables|Sounds|GetLaunchSound) "0, 0, 0" "0, 0, 0" 1.0 1.0 0.0 0 0 0 0)
  (Variables|ProjectilesSettings|SetStartLocation (Transformation|GetActorLocation))
  (Variables|Target|GetTarget
    (:then
      (CallFunction|RotatetoTarget))
    (:else)))

(event EventTick
  (params (DeltaSeconds :type Float%20%28single-precision%29))
  (if (>= (Math|Vector|VectorLength (- (Transformation|GetActorLocation) (Variables|ProjectilesSettings|GetStartLocation))) (Variables|ProjectilesSettings|GetMaxRange))
    (Actor|DestroyActor)))

(fn ConstructionScript
  (bind _projectilemovement (Variables|Default|GetProjectileMovement))
  (Transformation|SetWorldScale3D (Variables|Default|GetBoxCollision) (Variables|ProjectilesSettings|GetProjectileScale))
  (bind _output_get (Variables|/Script/Engine.ProjectileMovementComponent|SetInitialSpeed _projectilemovement (Variables|ProjectilesSettings|GetSpeed)))
  (Variables|/Script/Engine.ProjectileMovementComponent|SetMaxSpeed _projectilemovement _output_get)
  (Variables|Target|GetTarget
    (:then
      (if (Variables|ProjectilesSettings|GetIsHoming)
        (Variables|/Script/Engine.ProjectileMovementComponent|SetbIsHomingProjectile _projectilemovement true)
        (Variables|/Script/Engine.ProjectileMovementComponent|SetHomingTargetComponent _projectilemovement (Variables|/Script/Engine.Actor|GetRootComponent (Variables|Target|GetTarget)))))
    (:else)))