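; Procedural dungeon generator that builds a level-scaled layout of rooms, enemies and a boss, then places the player at its start.
; Random rooms attach recursively to open exits, with a short delay to reject overlapping ones.
; The room furthest from the start becomes the boss room, and leftover exits are walled off.
; Room events lock doors on entry and reopen them once enemies die, while dispatchers report room clears and boss defeat.
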(event Custom|SpawnStartRoom
  ;[0.1683 0.8148 1 0.502 35] SpawnStartRoom
  (Development|PrintString "Start Room" true true "(R=0.000000,G=0.660000,B=1.000000,A=1.000000)" 2e+02)
  (bind _returnvalue (Game|SpawnActorfromClass :Class "/Game/LoopFeeder/ProceduralDungeon/Rooms/BP_Dungeon_StartRoom.BP_Dungeon_StartRoom_C" :SpawnTransform (Math|Transform|MakeTransform (Variables|Default|GetDungeonWorldLocation) "0, 0, 0" "1.000000,1.000000,1.000000") :CollisionHandlingOverride "AlwaysSpawn" :TransformScaleMethod "MultiplyWithRoot" :Instigator 0))
  (bind _output_get (Variables|Default|SetStartRoom _returnvalue))
  (Variables|Default|SetExitsList (Components|GetChildrenComponents (Variables|/Game/LoopFeeder/ProceduralDungeon/Rooms/BP_Room_Base.BP_Room_Base_C|GetExit%20Folder _returnvalue) false))
  (CallFunction|AddingDoorstoRoom _output_get)
  (Utilities|Array|Add (Variables|Default|GetRoomInDungeon) _output_get)
  (CallFunction|SpawnNextRoom))

(event Custom|SpawnNextRoom
  ;[0.1683 0.8148 1 0.502 35] SpawnNextRoom
  (bind _output_get (Variables|Default|SetSelectedExit (.OutItem (Utilities|Array|Random (Variables|Default|GetExitsList)))))
  (Utilities|Array|RemoveItem (Variables|Default|GetExitsList) (Variables|Default|GetSelectedExit))
  (bind _returnvalue (Game|SpawnActorfromClass (.OutItem (Utilities|Array|Random (Variables|Default|GetRoomList))) (Math|Transform|MakeTransform (Transformation|GetWorldLocation _output_get) (Transformation|GetWorldRotation _output_get) "1.000000,1.000000,1.000000") "AlwaysSpawn" "MultiplyWithRoot" 0 0))
  (bind _asbp_room_base (Utilities|Casting|CastToBP_Room_Base _returnvalue))
  (bind _output_get_2 (Variables|Default|SetBP_Room_Base _asbp_room_base))
  (EventDispatchers|BindEventtoOnRoomEntered _output_get_2 (EventDispatchers|CreateEvent :!event Custom|RoomEntered))
  (Utilities|Array|Add (Variables|Default|GetRoomInDungeon) _output_get_2)
  (Utilities|FlowControl|Delay 0.2)
  (if (not (Variables|/Game/LoopFeeder/ProceduralDungeon/Rooms/BP_Room_Base.BP_Room_Base_C|GetIsOverlapping (Variables|Default|GetBP_Room_Base)))
    (bind _output_get_3 (Variables|Default|SetCurrentRoom (Variables|Default|GetBP_Room_Base)))
    (CallFunction|EnemySpawner _output_get_3)
    (CallFunction|AddingDoorstoRoom _output_get_3)
    (Utilities|Array|AppendArray (Variables|Default|GetExitsList) (Components|GetChildrenComponents (Variables|/Game/LoopFeeder/ProceduralDungeon/Rooms/BP_Room_Base.BP_Room_Base_C|GetExit%20Folder (Variables|Default|GetCurrentRoom)) false))
    (bind _result (Math|Integer|DecrementInt (Variables|Default|GetRoomAmount))
      (:%20%20
        (bind _output_get_4 (Variables|Default|SetRoomAmount _result))
        (if (> _output_get_4 0)
          (CallFunction|SpawnNextRoom)
          (else
            (bind _furthestroom (CallFunction|FindFurthestRoom))
            (Development|PrintString (Utilities|GetDisplayName _furthestroom) true true "(R=0.000000,G=1.000000,B=0.041006,A=1.000000)" 2e+02)
            (bind _returnvalue_2 (Game|SpawnActorfromClass :Class "/Game/LoopFeeder/ProceduralDungeon/Rooms/BP_Dungeon_BossRoom.BP_Dungeon_BossRoom_C" :SpawnTransform (Math|Transform|MakeTransform (Transformation|GetActorLocation _furthestroom) (Transformation|GetActorRotation _furthestroom) "1.000000,1.000000,1.000000") :CollisionHandlingOverride "AlwaysSpawn" :TransformScaleMethod "MultiplyWithRoot" :Instigator 0))
            (Variables|Default|SetBoss%20Room _returnvalue_2)
            (Actor|DestroyActor (Variables|Default|GetFurthestRoom))
            (bind _returnvalue_3 (Game|SpawnActorfromClass "/Game/LoopFeeder/DamageSystem/Enemy/BP_Enemy_Boss.BP_Enemy_Boss_C" (Math|Transform|MakeTransform (Math|Vector|MakeVector (.x (Transformation|GetWorldLocation (Variables|/Game/LoopFeeder/ProceduralDungeon/Rooms/BP_Dungeon_BossRoom.BP_Dungeon_BossRoom_C|GetBossSpawn _returnvalue_2))) (.y (Transformation|GetWorldLocation (Variables|/Game/LoopFeeder/ProceduralDungeon/Rooms/BP_Dungeon_BossRoom.BP_Dungeon_BossRoom_C|GetBossSpawn _returnvalue_2))) 4e+02) (Transformation|GetWorldRotation (Variables|/Game/LoopFeeder/ProceduralDungeon/Rooms/BP_Dungeon_BossRoom.BP_Dungeon_BossRoom_C|GetBossSpawn _returnvalue_2)) "1.000000,1.000000,1.000000") "AlwaysSpawn" "MultiplyWithRoot" 0 0 0))
            (EventDispatchers|BindEventtoOnBossDead _returnvalue_3 (EventDispatchers|CreateEvent :!event Custom|BossDefeated))
            (CallFunction|PutWallonExits)
            (Variables|Default|SetDungeonComplete true)
            (Development|PrintString "set player location" true true "(R=1.000000,G=0.961930,B=0.000000,A=1.000000)" 2e+02)
            (Transformation|SetActorLocation (Variables|Default|GetBP_Player) (+ (Variables|Default|GetDungeonWorldLocation) "1500.000000,0.000000,50.000000") false false)
            (for _array_element (Variables|Default|GetRoomInDungeon)
              (bind _asbp_room_base_2 (Utilities|Casting|CastToBP_Room_Base _array_element))
              (for _array_element_2 (Variables|/Game/LoopFeeder/ProceduralDungeon/Rooms/BP_Room_Base.BP_Room_Base_C|GetRoomDoorsList _asbp_room_base_2)
                (Collision|SetActorEnableCollision _array_element_2 false)
                (Rendering|SetActorHiddenInGame _array_element_2 true)))))))
    (else
      (Actor|DestroyActor (Variables|Default|GetBP_Room_Base))
      (CallFunction|SpawnNextRoom))))

(event Custom|RoomEntered
  (params (RoomEntered :type BP%20Room%20Base%20Object%20Reference))
  (for _array_element (Variables|/Game/LoopFeeder/ProceduralDungeon/Rooms/BP_Room_Base.BP_Room_Base_C|GetRoomDoorsList RoomEntered)
    (Collision|SetActorEnableCollision _array_element true)
    (Rendering|SetActorHiddenInGame _array_element false)))

(event Custom|ResetIfTooLong
  (if (not (Variables|Default|GetDungeonComplete))
    (Game|OpenLevel(byName) "Lvl_ThirdPerson")))

(event Custom|PutWallOnExits
  ;[0.1683 0.8148 1 0.502 35] Put Walls On Exits
  (for _array_element (Variables|Default|GetExitsList)
    (Game|SpawnActorfromClass "/Game/LoopFeeder/ProceduralDungeon/Rooms/BP_WallForHoles.BP_WallForHoles_C" (Math|Transform|MakeTransform (Transformation|GetWorldLocation _array_element) (Transformation|GetWorldRotation _array_element) "1.000000,1.000000,1.000000") "AlwaysSpawn" "MultiplyWithRoot" 0 0)))

(event Custom|SpawnPlayer
  (bind _returnvalue (Game|SpawnActorfromClass "/Game/LoopFeeder/DamageSystem/Player/BP_Player.BP_Player_C" (Math|Transform|MakeTransform "1500.000000,0.000000,50.000000" "0, 0, 0" "1.000000,1.000000,1.000000") "AlwaysSpawn" "MultiplyWithRoot" 0 "NewEnumerator1" 0 0))
  (Variables|Default|SetBP_Player _returnvalue))

(event Custom|EnemySpawner
  (params (CurrentRoom :type BP%20Room%20Base%20Object%20Reference))
  (bind _floor_spawn_points_folder (Variables|/Game/LoopFeeder/ProceduralDungeon/Rooms/BP_Room_Base.BP_Room_Base_C|GetFloor%20Spawn%20Points%20Folder CurrentRoom))
  (bind _children (Components|GetChildrenComponents _floor_spawn_points_folder false))
  ;[0.2737 1 0.3358 0.502 35] EnemySpawner
  (Utilities|Array|Shuffle _children)
  (bind _array_element (Utilities|Array|ForEachLoopwithBreak _children :!label _label)
    (:LoopBody
      (bind _returnvalue (Game|SpawnActorfromClass "/Game/LoopFeeder/DamageSystem/Enemy/BP_Enemy_Base.BP_Enemy_Base_C" (Math|Transform|MakeTransform (+ (Transformation|GetWorldLocation _array_element) "0.000000,0.000000,150.000000") "0, 0, 0" "1.000000,1.000000,1.000000") "AlwaysSpawn" "MultiplyWithRoot" 0 CurrentRoom 0))
      (bind _output_get (Variables|Default|SetSpawnedEnemy _returnvalue))
      (EventDispatchers|BindEventtoOnEnemyDead _output_get (EventDispatchers|CreateEvent :!event Custom|HandleEnemyDied))
      (Variables|/Game/LoopFeeder/DamageSystem/Enemy/BP_Enemy_Base.BP_Enemy_Base_C|SetOwningRoom (Variables|Default|GetSpawnedEnemy) (Variables|Default|GetCurrentRoom))
      (Utilities|Array|Add (Variables|/Game/LoopFeeder/ProceduralDungeon/Rooms/BP_Room_Base.BP_Room_Base_C|GetSpawnedEnemies (Variables|Default|GetCurrentRoom)) (Variables|Default|GetSpawnedEnemy))
      (if (> (Variables|Default|GetEnemySpawnAmount) 0)
        (Math|Integer|DecrementInt (Variables|Default|GetEnemySpawnAmount))
        (else
          (goto _label Break))))))

(event Custom|HandleEnemyDied
  (params (EnemyDead :type BP%20Enemy%20Base%20Object%20Reference))
  (bind _output_get (Variables|Default|SetEnemyDead EnemyDead))
  (Utilities|Array|RemoveItem (Variables|/Game/LoopFeeder/ProceduralDungeon/Rooms/BP_Room_Base.BP_Room_Base_C|GetSpawnedEnemies (Variables|/Game/LoopFeeder/DamageSystem/Enemy/BP_Enemy_Base.BP_Enemy_Base_C|GetOwningRoom _output_get)) (Variables|Default|GetEnemyDead))
  (if (<= (Utilities|Array|Length (Variables|/Game/LoopFeeder/ProceduralDungeon/Rooms/BP_Room_Base.BP_Room_Base_C|GetSpawnedEnemies (Variables|/Game/LoopFeeder/DamageSystem/Enemy/BP_Enemy_Base.BP_Enemy_Base_C|GetOwningRoom _output_get))) 0)
    (CallFunction|RoomCleared (Variables|/Game/LoopFeeder/DamageSystem/Enemy/BP_Enemy_Base.BP_Enemy_Base_C|GetOwningRoom _output_get))
    (Development|PrintString "RoomCleared" true true "(R=0.000000,G=0.660000,B=1.000000,A=1.000000)" 2e+01)))

(event Custom|RoomCleared
  (params (Room :type BP%20Room%20Base%20Object%20Reference))
  (Variables|/Game/LoopFeeder/ProceduralDungeon/Rooms/BP_Room_Base.BP_Room_Base_C|SetIsCleared Room true)
  (for _array_element (Variables|/Game/LoopFeeder/ProceduralDungeon/Rooms/BP_Room_Base.BP_Room_Base_C|GetRoomDoorsList Room)
    (Collision|SetActorEnableCollision _array_element false)
    (Rendering|SetActorHiddenInGame _array_element true))
  (Default|CallOnRoomCleared Room))

(event Custom|BossDefeated
  (Default|CallOnBossDefeated))

(event Custom|GenerateDungeon
  (Development|PrintString "GenerateDungeon" true true "(R=1.000000,G=0.007620,B=0.000080,A=1.000000)" 2e+01)
  (Math|Integer|IncrementInt (Variables|DungeonLevel|GetDungeonLevel)
    (:%20%20
      (Variables|Default|SetRoomAmount (+ 5 (* (Variables|DungeonLevel|GetDungeonLevel) 2)))
      (Variables|Default|SetEnemySpawnAmount (+ 1 (Variables|DungeonLevel|GetDungeonLevel)))
      (Utilities|Array|Clear (Variables|Default|GetExitsList))
      (Utilities|Array|Clear (Variables|Default|GetOverlappingRoomList))
      (Utilities|Array|Clear (Variables|Default|GetRoomInDungeon))
      (Variables|Default|SetDungeonComplete false)
      (Variables|Default|SetDungeonWorldLocation (+ (Variables|Default|GetDungeonLocationOffset) (Variables|Default|GetDungeonWorldLocation)))
      (CallFunction|SpawnStartRoom))))

(event Custom|AddingDoorsToRoom
  (params (Room :type BP%20Room%20Base%20Object%20Reference))
  (for _array_element (Components|GetChildrenComponents (Variables|/Game/LoopFeeder/ProceduralDungeon/Rooms/BP_Room_Base.BP_Room_Base_C|GetExit%20Folder Room) false)
    (bind _returnvalue (Game|SpawnActorfromClass "/Game/LoopFeeder/ProceduralDungeon/Rooms/BP_Doors.BP_Doors_C" (Math|Transform|MakeTransform (Transformation|GetWorldLocation _array_element) (Transformation|GetWorldRotation _array_element) "1.000000,1.000000,1.000000") "AlwaysSpawn" "MultiplyWithRoot" Room 0))
    (bind _asbp_room_base (Utilities|Casting|CastToBP_Room_Base (Components|GetOwner _returnvalue)))
    (Utilities|Array|Add (Variables|/Game/LoopFeeder/ProceduralDungeon/Rooms/BP_Room_Base.BP_Room_Base_C|GetRoomDoorsList _asbp_room_base) _returnvalue)))

(event EventBeginPlay
  (CallFunction|GenerateDungeon)
  (CallFunction|SpawnPlayer))

(fn ConstructionScript)

(fn FindFurthestRoom
  (for _array_element (Variables|Default|GetRoomInDungeon)
    (bind _output_get (LocalVariables|SetRoomForDistance _array_element))
    (bind _output_get_2 (LocalVariables|SetDistanceWithStartRoom (Math|Vector|Distance(Vector) (Transformation|GetActorLocation _output_get) (Transformation|GetActorLocation (Variables|Default|GetStartRoom)))))
    (if (> _output_get_2 (LocalVariables|GetMaxDistance))
      (LocalVariables|SetMaxDistance (LocalVariables|GetDistanceWithStartRoom))
      (Variables|Default|SetFurthestRoom (LocalVariables|GetRoomForDistance))))
  (return (Variables|Default|GetFurthestRoom)))