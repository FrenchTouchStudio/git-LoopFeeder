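; Base projectile Blueprint that moves at a configurable speed and handles its own launch and impact feedback.
; The construction script sets both the initial and max speed of ProjectileMovement from the Speed variable.
; BeginPlay spawns the launch effect at the collision box but plays the launch sound at world origin.
; A box hit calls OnProjectileImpact with the actor and hit result, plays impact effect and sound, then destroys the projectile.
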(event OnComponentHit(BoxCollision)
  (params (HitComponent :type Primitive%20Component%20Object%20Reference) (OtherActor :type Actor%20Object%20Reference) (OtherComp :type Primitive%20Component%20Object%20Reference) (NormalImpulse :type Vector :default "0, 0, 0") (Hit :type Hit%20Result%20Structure%20%28by%20ref%29))
  (bind _location (Collision|BreakHitResult Hit))
  (Default|CallOnProjectileImpact OtherActor Hit)
  (Effects|SpawnEmitteratLocation (Variables|Effects|GetImpactEffect) _location "0, 0, 0" (Variables|Effects|GetImpactEffectScale))
  (Audio|PlaySoundatLocation (Variables|Sounds|GetImpactSound) _location "0, 0, 0" 1.0 1.0 0.0 0 0 0 0)
  (Actor|DestroyActor))

(event EventBeginPlay
  (Effects|SpawnEmitteratLocation (Variables|Effects|GetLaunchEffect) (Transformation|GetWorldLocation (Variables|Default|GetBoxCollision)))
  (Audio|PlaySoundatLocation (Variables|Sounds|GetLaunchSound) "0, 0, 0" "0, 0, 0" 1.0 1.0 0.0 0 0 0 0))

(fn ConstructionScript
  (bind _projectilemovement (Variables|Default|GetProjectileMovement))
  (bind _output_get (Variables|/Script/Engine.ProjectileMovementComponent|SetInitialSpeed _projectilemovement (Variables|ProjectilesSettings|GetSpeed)))
  (Variables|/Script/Engine.ProjectileMovementComponent|SetMaxSpeed _projectilemovement _output_get))